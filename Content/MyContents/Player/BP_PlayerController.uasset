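; Player controller for a neon-themed runner that manages UI, a game timer and difficulty values.
; BeginPlay shows the lobby widget, prepares main and game-over widgets, spawns an overlay character below the world and caches the PlayerStart.
; Tick watches the GameMode's GameStart flag, using paired DoOnce gates to start or clear a one-second counter.
; IncreaseDifficulty raises pawn speed and capped obstacle and drone spawn chances; EndGame swaps lobby for game-over UI.
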(event `self.ReceiveBeginPlay`
  (bind _returnvalue (`|CreateWidget` "/Game/MyContents/UI/WBP_LobbyUI.WBP_LobbyUI_C"))
  (bind _output_get (set `self.LobbyUIWidget` _returnvalue))
  (`UserWidget.AddToViewport` _output_get 1)
  (bind _returnvalue_2 (`|SpawnActorFromClass` "/Game/MyContents/UI/BP_OverlayCharacter.BP_OverlayCharacter_C" (`KismetMathLibrary.MakeTransform` (0.0 0.0 -2000.0)) "Undefined" "MultiplyWithRoot" null null))
  (set `self.OverlayChracter` _returnvalue_2)
  (bind _returnvalue_3 (`|CreateWidget` "/Game/MyContents/UI/WBP_MainUI.WBP_MainUI_C"))
  (set `self.MainUIWidget` _returnvalue_3)
  (bind _returnvalue_4 (`|CreateWidget` "/Game/MyContents/UI/WBP_GameOver.WBP_GameOver_C"))
  (set `self.GameOverWidget` _returnvalue_4)
  (bind _outactors (`GameplayStatics.GetAllActorsOfClass` "/Script/Engine.PlayerStart"))
  (set `self.PlayerStart` (`|GetArrayItem` _outactors)))

(event `self.ReceiveTick`
  (params (DeltaSeconds :type "Float (single-precision)"))
  (bind _timerhandle (`self.TimerHandle`))
  (bind _asbp_neon_game_mode (cast `/Game/MyContents/BP_NeonGameMode` (`GameplayStatics.GetGameMode`)))
  (if (`/Game/MyContents/BP_NeonGameMode.bGameStart` _asbp_neon_game_mode)
    (`/Engine/EditorBlueprintResources/StandardMacros.DoOnce` false :!label _label
      (:`Completed`
        (bind _returnvalue (`KismetSystemLibrary.K2_SetTimerDelegate` (delegate `GameTimer`) 1.0 true))
        (set `self.TimerHandle` _returnvalue)
        (goto _label_2 :!via `Reset`)))
    (else
      (`/Engine/EditorBlueprintResources/StandardMacros.DoOnce` true :!label _label_2
        (:`Completed`
          (if (`KismetSystemLibrary.K2_IsValidTimerHandle` _timerhandle)
            (`KismetSystemLibrary.K2_ClearAndInvalidateTimerHandle` _timerhandle)
            (goto _label :!via `Reset`)))))))

(event `GameTimer`
  (bind _result (`/Engine/EditorBlueprintResources/StandardMacros.IncrementInt` (`self.GamePlayTimer`))
    (:`  `
      (if (== (mod _result 10) 0)
        _))))

(fn `EndGame`
  (`Widget.RemoveFromParent` (`self.LobbyUIWidget`))
  (`UserWidget.AddToViewport` (`self.GameOverWidget`) 0))

(fn `IncreaseDifficulty`
  (`|ExecutionSequence`
    (:`then_0`
      (bind _asbp_player_character (cast `/Game/MyContents/Player/BP_PlayerCharacter` (`self.K2_GetPawn`)))
      (`/Game/MyContents/Player/BP_PlayerCharacter.AddSpeed` _asbp_player_character 50.0))
    (:`then_1`
      (bind _output_get (set `self.ObstacleSpawnChance` (+ (`self.ObstacleSpawnChance`) 5.0)))
      (if (>= _output_get 1.0)
        (set `self.ObstacleSpawnChance` 1.0)))
    (:`then_2`
      (bind _output_get_2 (set `self.EnemyDroneSpawnChance` (+ (`self.EnemyDroneSpawnChance`) 5.0)))
      (if (>= _output_get_2 1.0)
        (set `self.EnemyDroneSpawnChance` 1.0)))))

(fn `UserConstructionScript`)