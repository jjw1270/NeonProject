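; Enemy drone that hovers up and down between Z limits, turns to face the player and shoots at them.
; Tick drives the bobbing and aiming, while a looping timer fires projectiles once the game has started, if a line trace hits the living player.
; Damage alters its hologram dynamic material, and zero life triggers an explosion and sound.
; It destroys itself silently once the player passes it along X.
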(event `self.ReceiveBeginPlay`
  (bind _asbp_player_character (cast `/Game/MyContents/Player/BP_PlayerCharacter` (`Controller.K2_GetPawn` (`GameplayStatics.GetPlayerController` 0))))
  (set `self.PlayerCharacter` _asbp_player_character)
  (`self.SetLife` (`self.MaxLife`))
  (`self.SetMoveLocation`)
  (bind _returnvalue (`KismetSystemLibrary.K2_SetTimer` null "SearchAndShoot" (`self.ShootingDelay`) true))
  (set `self.SearchAndShootHandle` _returnvalue))

(event `self.ReceiveTick`
  (params (DeltaSeconds :type "Float (single-precision)"))
  (`self.Rotate`)
  (`self.Move`))

(fn `DestroySelf`
  (params (Damaged :type Boolean))
  (bind _searchandshoothandle (`self.SearchAndShootHandle`))
  (if Damaged
    (`GameplayStatics.SpawnEmitterAtLocation` "/Game/Realistic_Starter_VFX_Pack_Vol2/Particles/Explosion/P_Explosion_Big_A.P_Explosion_Big_A" (`self.K2_GetActorLocation`))
    (bind _asbp_neon_game_mode (cast `/Game/MyContents/BP_NeonGameMode` (`GameplayStatics.GetGameMode`)))
    (`/Game/MyContents/BP_NeonGameMode.PlaySound` _asbp_neon_game_mode "/Game/SoundAssets/Shoot/Sci_Fi_Grenade_5.Sci_Fi_Grenade_5" (`self.K2_GetActorLocation`) 1.0 false))
  (if (`KismetSystemLibrary.K2_IsValidTimerHandle` _searchandshoothandle)
    (`KismetSystemLibrary.K2_ClearAndInvalidateTimerHandle` _searchandshoothandle))
  (`self.K2_DestroyActor`))

(fn `Move`
  (bind (_returnvalue_x _returnvalue_y _returnvalue_z) (`KismetMathLibrary.BreakVector` (`self.K2_GetActorLocation`)))
  (bind (_returnvalue_x_2 _returnvalue_y_2 _returnvalue_z_2) (`KismetMathLibrary.BreakVector` (`self.K2_GetActorLocation`)))
  (if (`self.bIsGoingUp`)
    (if (< _returnvalue_z (`self.MaxZDist`))
      (`self.K2_AddActorWorldOffset` (0.0 0.0 1.5))
      (else
        (set `self.bIsGoingUp` false)))
    (elif (> _returnvalue_z_2 (`self.MinZDist`))
      (`self.K2_AddActorWorldOffset` (0.0 0.0 -1.5))
      (else
        (set `self.bIsGoingUp` true)))))

(fn `Rotate`
  (bind _playercharacter (`self.PlayerCharacter`)
    (:`then`
      (`self.K2_SetActorRotation` (`KismetMathLibrary.FindLookAtRotation` (`self.K2_GetActorLocation`) (`SceneComponent.K2_GetComponentLocation` (`/Game/MyContents/Player/BP_PlayerCharacter.ProjectileSpawnPoint` _playercharacter)))))
    (:`else`)))

(fn `SearchAndShoot`
  (locals (ShootPos :type "Vector Structure" :default (0.0 0.0 0.0)) (TargetPos :type "Vector Structure" :default (0.0 0.0 0.0)))
  (bind _playercharacter (`self.PlayerCharacter`))
  (bind _returnvalue (`SceneComponent.K2_GetComponentLocation` (`self.ShootPosition`)))
  (bind _returnvalue_2 (`SceneComponent.K2_GetComponentLocation` (`self.ShootPosition`)))
  (bind _asbp_neon_game_mode (cast `/Game/MyContents/BP_NeonGameMode` (`GameplayStatics.GetGameMode`)))
  (if (`/Game/MyContents/BP_NeonGameMode.bGameStart` _asbp_neon_game_mode)
    (bind _playercharacter_2 (`self.PlayerCharacter`)
      (:`then`
        (bind _returnvalue_3 (`self.K2_GetActorLocation` _playercharacter_2))
        (bind _returnvalue_x (`KismetMathLibrary.BreakVector` (- _returnvalue _returnvalue_3)))
        (if (> _returnvalue_x -30.0)
          (bind _outhit (`KismetSystemLibrary.LineTraceSingle` _returnvalue _returnvalue_3 "TraceTypeQuery2"))
          (bind (_bblockinghit _binitialoverlap _time _distance _location _impactpoint _normal _impactnormal _physmat _hitactor) (`GameplayStatics.BreakHitResult` _outhit))
          (if (and (> (`/Game/MyContents/Player/BP_PlayerCharacter.Life` _playercharacter) 0) (== _playercharacter _hitactor))
            (`|SpawnActorFromClass` "/Game/MyContents/Projectile/BP_EnemyProjectile.BP_EnemyProjectile_C" (`KismetMathLibrary.MakeTransform` _returnvalue_2 (`KismetMathLibrary.FindLookAtRotation` _returnvalue_2 _location)) "Undefined" "MultiplyWithRoot" null null))
          (else
            (`self.DestroySelf` false))))
      (:`else`))))

(fn `SetLife`
  (params (AddedHealth :type Integer))
  (bind _materialinst (`self.MaterialInst`))
  (bind _output_get (set `self.Life` (+ AddedHealth (`self.Life`))))
  (if (< _output_get (`self.MaxLife`))
    (`MaterialInstanceDynamic.SetScalarParameterValue` _materialinst "Width1" 0.15)
    (`MaterialInstanceDynamic.SetScalarParameterValue` _materialinst "Width2" 0.15)
    (if (<= (`self.Life`) 0)
      (`self.DestroySelf` true))))

(fn `SetMoveLocation`
  (if (`KismetMathLibrary.RandomBool`)
    (set `self.bIsGoingUp` true)
    (else
      (set `self.bIsGoingUp` false))))

(fn `UserConstructionScript`
  (bind _returnvalue (`PrimitiveComponent.CreateDynamicMaterialInstance` (`self.DroneSkeletalMesh`) 0 "/Game/MyContents/Materials/MI_HologramEnemyDrone.MI_HologramEnemyDrone" "None"))
  (set `self.MaterialInst` _returnvalue)
  (`PrimitiveComponent.SetMaterial` (`self.DroneSkeletalMesh`) 0 (`self.MaterialInst`)))