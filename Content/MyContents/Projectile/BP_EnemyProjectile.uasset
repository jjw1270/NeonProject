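; BP_EnemyProjectile is an enemy projectile that damages the player on impact and self-destructs after a fixed lifetime.
; BeginPlay caches the possessed BP_PlayerCharacter and starts the lifetime delay.
; Box hits branch on collision object type: Player calls SetLife on the cached character, while World Static and Destructible count as obstacles.
; Both outcomes spawn random impact sparks aligned to the surface normal, play a sound at world origin, then destroy the projectile.
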(event `self.ReceiveBeginPlay`
  (bind _asbp_player_character (cast `/Game/MyContents/Player/BP_PlayerCharacter` (`Controller.K2_GetPawn` (`GameplayStatics.GetPlayerController` 0))))
  (set `self.PlayerCharacter` _asbp_player_character)
  (`KismetSystemLibrary.Delay` 10.0)
  (`self.K2_DestroyActor`))

(event `self.Box.OnComponentHit`
  (params (HitComponent :type "PrimitiveComponent Object Reference") (OtherActor :type "Actor Object Reference") (OtherComp :type "PrimitiveComponent Object Reference") (NormalImpulse :type "Vector Structure") (Hit :type "HitResult Structure (by ref)"))
  (switch `ECollisionChannel` (`PrimitiveComponent.GetCollisionObjectType` OtherComp)
    (:`ECC_WorldStatic`
      (`self.HitObstacle` Hit :!label _label))
    (:`ECC_Destructible`
      (goto _label))
    (:`ECC_GameTraceChannel3`
      (`self.HitPlayer` Hit)))
  (`self.K2_DestroyActor`))

(fn `HitObstacle`
  (params (Hit :type "HitResult Structure (by ref)"))
  (bind (_bblockinghit _binitialoverlap _time _distance _location _impactpoint _normal _impactnormal) (`GameplayStatics.BreakHitResult` Hit))
  (`GameplayStatics.SpawnEmitterAtLocation` (`KismetArrayLibrary.Array_Random` (`self.EnemySparkes`)) _location (`KismetMathLibrary.MakeRotFromZ` _impactnormal))
  (`GameplayStatics.PlaySoundAtLocation` "/Engine/VREditor/Sounds/UI/Click_on_Button_Cue.Click_on_Button_Cue" (0.0 0.0 0.0) (struct) 1.0 1.0 0.0 null null null null) ; Play firing sound
)

(fn `HitPlayer`
  (params (Hit :type "HitResult Structure (by ref)"))
  (bind (_bblockinghit _binitialoverlap _time _distance _location _impactpoint _normal _impactnormal) (`GameplayStatics.BreakHitResult` Hit))
  (bind _playercharacter (`self.PlayerCharacter`)
    (:`then`
      (`/Game/MyContents/Player/BP_PlayerCharacter.SetLife` _playercharacter -1)
      (`GameplayStatics.SpawnEmitterAtLocation` (`KismetArrayLibrary.Array_Random` (`self.DefaultSparkes`)) _location (`KismetMathLibrary.MakeRotFromZ` _impactnormal))
      (`GameplayStatics.PlaySoundAtLocation` "/Engine/VREditor/Sounds/UI/Click_on_Button_Cue.Click_on_Button_Cue" (0.0 0.0 0.0) (struct) 1.0 1.0 0.0 null null null null) ; Play firing sound
    )
    (:`else`)))

(fn `UserConstructionScript`)