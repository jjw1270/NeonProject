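; Player projectile that damages obstacles and enemy drones on impact and expires after a short delay.
; Box hits branch on collision object type: static and destructible hits go to HitObstacle, enemy hits to HitEnemy plus a game-mode sound.
; Both handlers call SetLife on the target and spawn random sparks aligned to the impact normal before the projectile is destroyed.
; Tick also destroys it whenever the game mode's GameStart is false.
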(event `self.ReceiveBeginPlay`
  (`KismetSystemLibrary.Delay` 2.0)
  (`self.K2_DestroyActor`))

(event `self.Box.OnComponentHit`
  (params (HitComponent :type "PrimitiveComponent Object Reference") (OtherActor :type "Actor Object Reference") (OtherComp :type "PrimitiveComponent Object Reference") (NormalImpulse :type "Vector Structure") (Hit :type "HitResult Structure (by ref)"))
  (switch `ECollisionChannel` (`PrimitiveComponent.GetCollisionObjectType` OtherComp)
    (:`ECC_WorldStatic`
      (`self.HitObstacle` Hit :!label _label))
    (:`ECC_Destructible`
      (goto _label))
    (:`ECC_GameTraceChannel1`
      (`self.HitEnemy` Hit)
      (bind _asbp_neon_game_mode (cast `/Game/MyContents/BP_NeonGameMode` (`GameplayStatics.GetGameMode`)))
      (`/Game/MyContents/BP_NeonGameMode.PlaySound` _asbp_neon_game_mode "/Game/SoundAssets/Shoot/Sci_Fi_Grenade_5.Sci_Fi_Grenade_5" (`self.K2_GetActorLocation`) 1.0 false)))
  (`self.K2_DestroyActor`))

(event `self.ReceiveTick`
  (params (DeltaSeconds :type "Float (single-precision)"))
  (bind _asbp_neon_game_mode (cast `/Game/MyContents/BP_NeonGameMode` (`GameplayStatics.GetGameMode`)))
  (if (not (`/Game/MyContents/BP_NeonGameMode.bGameStart` _asbp_neon_game_mode))
    (`self.K2_DestroyActor`)))

(fn `HitEnemy`
  (params (Hit :type "HitResult Structure (by ref)"))
  (bind (_bblockinghit _binitialoverlap _time _distance _location _impactpoint _normal _impactnormal _physmat _hitactor) (`GameplayStatics.BreakHitResult` Hit))
  (bind _asbp_enemy_drone (cast `/Game/MyContents/EnemyDrone/BP_EnemyDrone` _hitactor)
    (:`then`
      (`/Game/MyContents/EnemyDrone/BP_EnemyDrone.SetLife` _asbp_enemy_drone -1))
    (:`CastFailed`
      _))
  (`GameplayStatics.SpawnEmitterAtLocation` (`KismetArrayLibrary.Array_Random` (`self.DefaultSparkes`)) _location (`KismetMathLibrary.MakeRotFromZ` _impactnormal)))

(fn `HitObstacle`
  (params (Hit :type "HitResult Structure (by ref)"))
  (bind (_bblockinghit _binitialoverlap _time _distance _location _impactpoint _normal _impactnormal _physmat _hitactor) (`GameplayStatics.BreakHitResult` Hit))
  (bind _asbp_obstacle_base (cast `/Game/MyContents/Obstacle/BP_ObstacleBase` _hitactor)
    (:`then`
      (`/Game/MyContents/Obstacle/BP_ObstacleBase.SetLife` _asbp_obstacle_base -1))
    (:`CastFailed`
      _))
  (`GameplayStatics.SpawnEmitterAtLocation` (`KismetArrayLibrary.Array_Random` (`self.DefaultSparkes`)) _location (`KismetMathLibrary.MakeRotFromZ` _impactnormal)))

(fn `UserConstructionScript`)