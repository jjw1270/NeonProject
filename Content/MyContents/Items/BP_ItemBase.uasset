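; BP_ItemBase is a collectible item, by name a base class, that reacts visually when a Player or Invincibility collision object overlaps its box.
; On overlap it spawns a scaled-up hit effect, removes its own item effect, then destroys the spawned effect after a short delay.
; A looping timer compares its X position with the cached player character's and destroys the actor once it falls far enough behind.
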(event `self.ReceiveBeginPlay`
  (bind _asbp_player_character (cast `/Game/MyContents/Player/BP_PlayerCharacter` (`Controller.K2_GetPawn` (`GameplayStatics.GetPlayerController` 0))))
  (set `self.PlayerCharacter` _asbp_player_character)
  (bind _returnvalue (`KismetSystemLibrary.K2_SetTimerDelegate` (delegate `CheckDistance`) 0.5 true))
  (set `self.CheckDistanceHandle` _returnvalue))

(event `CheckDistance`
  (bind _checkdistancehandle (`self.CheckDistanceHandle`))
  (bind _playercharacter (`self.PlayerCharacter`)
    (:`then`
      (bind _returnvalue_x (`KismetMathLibrary.BreakVector` (- (`self.K2_GetActorLocation`) (`self.K2_GetActorLocation` _playercharacter))))
      (if (< _returnvalue_x -400.0)
        (if (`KismetSystemLibrary.K2_IsValidTimerHandle` _checkdistancehandle)
          (`KismetSystemLibrary.K2_ClearAndInvalidateTimerHandle` _checkdistancehandle)
          (`self.K2_DestroyActor`))))
    (:`else`)))

(event `self.Box.OnComponentBeginOverlap`
  (params (OverlappedComponent :type "PrimitiveComponent Object Reference") (OtherActor :type "Actor Object Reference") (OtherComp :type "PrimitiveComponent Object Reference") (OtherBodyIndex :type Integer) (bFromSweep :type Boolean) (SweepResult :type "HitResult Structure (by ref)"))
  (switch `ECollisionChannel` (`PrimitiveComponent.GetCollisionObjectType` OtherComp)
    (:`ECC_GameTraceChannel2`
      _)
    (:`ECC_GameTraceChannel3`
      _))
  (bind _returnvalue (`NiagaraFunctionLibrary.SpawnSystemAtLocation` (`self.HitEffect`) (`self.K2_GetActorLocation`) (struct) (2.0 2.0 2.0) false))
  (`ActorComponent.K2_DestroyComponent` (`self.ItemEffect`))
  (`KismetSystemLibrary.Delay` 2.0)
  (`ActorComponent.K2_DestroyComponent` _returnvalue))

(fn `UserConstructionScript`)