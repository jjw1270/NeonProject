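; BP_Sector is a self-chaining map segment that fills itself with random obstacles and enemy drones.
; On BeginPlay it steps along X up to the next spawn point, rolling per step and per slot for up to three objects across Y, with drones at random heights.
; Player overlaps trigger spawning the next sector at MapSpawnPoint, or destroying this sector along with its tracked objects.
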(event `self.ReceiveBeginPlay`
  (`self.SpawnObjects` (`self.ObstacleDistance`) "/Game/MyContents/Obstacle/BP_ObstacleBase.BP_ObstacleBase_C")
  (`self.SpawnObjects` (`self.EnemyDistance`) "/Game/MyContents/EnemyDrone/BP_EnemyDrone.BP_EnemyDrone_C"))

(event `self.SpawnNextMapCollision.OnComponentBeginOverlap`
  (params (OverlappedComponent :type "PrimitiveComponent Object Reference") (OtherActor :type "Actor Object Reference") (OtherComp :type "PrimitiveComponent Object Reference") (OtherBodyIndex :type Integer) (bFromSweep :type Boolean) (SweepResult :type "HitResult Structure (by ref)"))
  (cast `/Game/MyContents/BP_PlayerCharacter` OtherActor)
  (`|SpawnActorFromClass` "BP_Sector_C" (`SceneComponent.K2_GetComponentToWorld` (`self.MapSpawnPoint`)) "Undefined" "MultiplyWithRoot" null null))

(event `self.DeleteThisMapCollision.OnComponentBeginOverlap`
  (params (OverlappedComponent :type "PrimitiveComponent Object Reference") (OtherActor :type "Actor Object Reference") (OtherComp :type "PrimitiveComponent Object Reference") (OtherBodyIndex :type Integer) (bFromSweep :type Boolean) (SweepResult :type "HitResult Structure (by ref)"))
  (cast `/Game/MyContents/BP_PlayerCharacter` OtherActor)
  (for _array_element (`self.Objects`)
    (`self.K2_DestroyActor` _array_element))
  (`self.K2_DestroyActor`))

(fn `UserConstructionScript`)