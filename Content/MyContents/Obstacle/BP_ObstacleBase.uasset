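; Base obstacle actor that spawns with a random height and removes itself once the player has moved past it along X.
; On BeginPlay it picks a Z scale from a preset list, randomly raising the smaller-index variants to an elevated position.
; A looping timer compares its X position with the player's and calls DestroySelf, which skips actor destruction when flagged as damaged.
; SetLife is an empty stub.
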(event `self.ReceiveBeginPlay`
  (bind _asbp_player_character (cast `/Game/MyContents/BP_PlayerCharacter` (`Controller.K2_GetPawn` (`GameplayStatics.GetPlayerController` 0))))
  (set `self.PlayerCharacter` _asbp_player_character)
  (`self.SetRandomScale`)
  (`self.SetRandomLocation`)
  (bind _returnvalue (`KismetSystemLibrary.K2_SetTimerDelegate` (delegate `CheckDistance`) 0.1 true))
  (set `self.CheckDistanceHandle` _returnvalue))

(event `CheckDistance`
  (bind _playercharacter (`self.PlayerCharacter`)
    (:`then`
      (bind _returnvalue_x (`KismetMathLibrary.BreakVector` (- (`self.K2_GetActorLocation`) (`self.K2_GetActorLocation` _playercharacter))))
      (if (< _returnvalue_x 0.0)
        (`self.DestroySelf` false)))
    (:`else`)))

(fn `DestroySelf`
  (params (Damaged :type Boolean))
  (bind _checkdistancehandle (`self.CheckDistanceHandle`))
  (if (`KismetSystemLibrary.K2_IsValidTimerHandle` _checkdistancehandle)
    (`KismetSystemLibrary.K2_ClearAndInvalidateTimerHandle` _checkdistancehandle)
    (if (not Damaged)
      (`self.K2_DestroyActor`))))

(fn `SetLife`)

(fn `UserConstructionScript`)