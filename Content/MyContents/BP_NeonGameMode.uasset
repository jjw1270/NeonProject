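; BP_NeonGameMode is a game mode Blueprint that manages background music and provides sound playback helpers.
; BeginPlay starts a lobby track, and once GameStart is set, Tick stops it and spawns a random track from BGMs.
; Tick then polls the current track, picking another random one whenever it is not playing.
; PlaySound spawns 2D or positional audio, while PlaySoundRandom plays a random entry at a location.
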(event `self.ReceiveBeginPlay`
  (bind _returnvalue (`GameplayStatics.SpawnSound2D` "/Game/SoundAssets/BGM/04_-_Lufus_-_Space_Time.04_-_Lufus_-_Space_Time" 0.5 1.0 0.0 null))
  (set `self.LobbyBGM` _returnvalue))

(event `self.ReceiveTick`
  (params (DeltaSeconds :type "Float (single-precision)"))
  (bind _lobbybgm (`self.LobbyBGM`))
  (if (`self.bGameStart`)
    (`/Engine/EditorBlueprintResources/StandardMacros.IsValid` _lobbybgm
      (:`Is Valid`
        (`AudioComponent.Stop` _lobbybgm)
        (bind _returnvalue (`GameplayStatics.SpawnSound2D` (`KismetArrayLibrary.Array_Random` (`self.BGMs`)) 0.5 1.0 0.0 null :!label _label))
        (set `self.NowPlayingBGM` _returnvalue))
      (:`Is Not Valid`
        (if (not (`AudioComponent.IsPlaying` (`self.NowPlayingBGM`)))
          (goto _label))))))

(fn `PlaySound`
  (params (Sound :type "SoundBase Object Reference") (Location :type "Vector Structure") (Volume :type "Float (single-precision)" :default 1.0) (`2D` :type Boolean))
  (if `2D`
    (`GameplayStatics.SpawnSound2D` Sound Volume 1.0 0.0 null)
    (else
      (`GameplayStatics.SpawnSoundAtLocation` Sound Location (struct) Volume 1.0 0.0 null null))))

(fn `PlaySoundRandom`
  (params (Sound :type "Array of SoundBase Object Reference") (Location :type "Vector Structure") (Volume :type "Float (single-precision)" :default 1.0))
  (`GameplayStatics.SpawnSoundAtLocation` (`KismetArrayLibrary.Array_Random` Sound) Location (struct) Volume 1.0 0.0 null null))

(fn `UserConstructionScript`)